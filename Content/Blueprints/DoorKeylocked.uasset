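; Locked door actor that opens when the player enters its trigger box while holding the door key.
; BeginPlay caches the BP_Player reference, and the box overlap checks that actor's DoorKey flag.
; A DoOnce gate fires the opening and a sound a single time, with no closing logic.
; The DoorOpen timeline drives the Platform component's relative Z location to move the door.
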(event `self.ReceiveBeginPlay`
  (bind _asbp_player (cast `/Game/Blueprints/BP_Player` (`GameplayStatics.GetPlayerCharacter` 0)))
  (set `self.As BP Player` _asbp_player))

(event `OpenDoor`
  (bind (_direction _newtrack_0) (`Timeline|DoorOpen`)
    (:`Update`
      (`SceneComponent.K2_SetRelativeLocation` (`self.Platform`) (`KismetMathLibrary.MakeVector` 0.0 0.0 (.z _newtrack_0)) false false))))

(event `self.Box.OnComponentBeginOverlap`
  (params (OverlappedComponent :type "PrimitiveComponent Object Reference") (OtherActor :type "Actor Object Reference") (OtherComp :type "PrimitiveComponent Object Reference") (OtherBodyIndex :type Integer) (bFromSweep :type Boolean) (SweepResult :type "HitResult Structure (by ref)"))
  (bind _as_bp_player (`self.As BP Player`))
  (if (== OtherActor _as_bp_player)
    (if (== (`/Game/Blueprints/BP_Player.DoorKey` _as_bp_player) true)
      (`/Engine/EditorBlueprintResources/StandardMacros.DoOnce` false
        (:`Completed`
          (`self.OpenDoor`)
          (`GameplayStatics.PlaySoundAtLocation` null (`self.K2_GetActorLocation`) (struct) 1.0 1.0 0.0 null null null null))))))

(fn `UserConstructionScript`)