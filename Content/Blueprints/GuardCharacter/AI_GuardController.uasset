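; AI controller for guard enemies that runs the BT_Guard behavior tree and feeds AI perception results into its blackboard.
; Sight and damage stimuli share one path that requires the player actor, setting CanSeePlayer from sensing success and TargetLocation from the player's position.
; Hearing does no player check: loud stimuli count as seeing the player at the noise location, while quieter ones set CanHearPlayer and AudioContactLocation.
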(event `self.ReceiveBeginPlay`
  (`self.RunBehaviorTree` "/Game/Blueprints/GuardCharacter/BT_Guard.BT_Guard")
  (bind _asbp_guard_enemy (cast `/Game/Blueprints/GuardCharacter/BP_GuardEnemy` (`self.K2_GetPawn`)))
  (set `self.MyGuardChar` _asbp_guard_enemy))

(event `self.AIPerception.OnTargetPerceptionUpdated`
  (params (Actor :type "Actor Object Reference") (Stimulus :type "AIStimulus Structure"))
  (bind (_age _expirationage _strength _stimuluslocation _receiverlocation _tag _bsuccessfullysensed) (break `AIStimulus` Stimulus))
  (bind _returnvalue (`AIBlueprintHelperLibrary.GetBlackboard` null))
  (bind _returnvalue_2 (`AIBlueprintHelperLibrary.GetBlackboard` null))
  (bind _returnvalue_3 (`AIBlueprintHelperLibrary.GetBlackboard` null))
  (bind _returnvalue_4 (> _strength 0.6))
  (bind _returnvalue_5 (`AIPerceptionSystem.GetSenseClassForStimulus` Stimulus))
  (switch `string` (`KismetSystemLibrary.GetClassDisplayName` _returnvalue_5)
    (:`AISense_Sight`
      (`KismetSystemLibrary.PrintString` "VISUAL CONTACT" false)
      (bind _asbp_player (cast `/Game/Blueprints/BP_Player` Actor :!label _label))
      (`BlackboardComponent.SetValueAsBool` _returnvalue_3 "CanSeePlayer" (`.bSuccessfullySensed` (break `AIStimulus` Stimulus)))
      (`BlackboardComponent.SetValueAsVector` _returnvalue_3 "TargetLocation" (`Pawn.GetNavAgentLocation` _asbp_player)))
    (:`AISense_Hearing`
      (`KismetSystemLibrary.PrintString` "AUDIO CONTACT" false)
      (if _returnvalue_4
        (`BlackboardComponent.SetValueAsBool` _returnvalue_2 "CanSeePlayer" _returnvalue_4)
        (`BlackboardComponent.SetValueAsVector` _returnvalue_2 "TargetLocation" _stimuluslocation)
        (else
          (`BlackboardComponent.SetValueAsBool` _returnvalue "CanHearPlayer" _bsuccessfullysensed)
          (`BlackboardComponent.SetValueAsVector` _returnvalue "AudioContactLocation" _stimuluslocation))))
    (:`AISense_Damage`
      (`KismetSystemLibrary.PrintString` "DAMAGE CONTACT" false)
      (goto _label))))

(fn `UserConstructionScript`)